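; BP_Turret is an enemy turret that shoots fireballs when it sees the player character and can be frozen.
; PawnSensing sightings of BP_ThirdPersonCharacter spawn a scaled-down BP_FireBall at BulletSpawner after a short delay, unless Death is already set.
; The Freezer event sets Death, swaps StaticMesh to a chamfered cube and applies ice materials.
; The look-at rotation nodes are disconnected, so this graph never aims the turret.
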(event `self.PawnSensing.OnSeePawn`
  (params (Pawn :type "Pawn Object Reference"))
  (bind (_returnvalue_location _returnvalue_rotation) (`KismetMathLibrary.BreakTransform` (`SceneComponent.K2_GetComponentToWorld` (`self.BulletSpawner`))))
  (if (not (`self.Death?`))
    (cast `/Game/ThirdPerson/Blueprints/BP_ThirdPersonCharacter` Pawn)
    (`KismetSystemLibrary.Delay` 1.0)
    (`|SpawnActorFromClass` "/Game/Octavio/Bullet/BP_FireBall.BP_FireBall_C" (`KismetMathLibrary.MakeTransform` _returnvalue_location _returnvalue_rotation (0.6 0.6 0.6)) "AlwaysSpawn" "OverrideRootScale" null null)))

(event `Freezer`
  (bind _staticmesh (`self.StaticMesh`))
  (set `self.Death?` true)
  (`StaticMeshComponent.SetStaticMesh` _staticmesh "/Game/LevelPrototyping/Meshes/SM_ChamferCube.SM_ChamferCube")
  (`PrimitiveComponent.SetMaterial` _staticmesh 0 "/Game/Bishop/M_Ice_Inst.M_Ice_Inst")
  (`PrimitiveComponent.SetMaterial` (`self.Turret`) 0 "/Game/Bishop/M_Ice.M_Ice"))

(fn `UserConstructionScript`)